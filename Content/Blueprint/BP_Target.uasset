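; BP_Target is a target actor that swings into position, can be knocked down and awards a point to the game mode.
; Fight plays a timeline that lerps the scene component's rotation through 90 degrees, with a piston sound at the player's location.
; Down spawns an explosion and reverses that timeline, while PointUP increments and prints the FirstPersonGameMode score.
; Down and PointUP each use a DoOnce that is never reset.
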(event Custom|Event%20PointUP
  (bind _gmref (Variables|Default|GetGMRef))
  ;[1 1 1] Point up
  (Utilities|FlowControl|DoOnce false
    (:Completed
      (Variables|/Game/FirstPersonBP/Blueprints/FirstPersonGameMode.FirstPersonGameMode_C|SetPoint _gmref (+ (Variables|/Game/FirstPersonBP/Blueprints/FirstPersonGameMode.FirstPersonGameMode_C|GetPoint _gmref) 1))
      (Development|PrintString (Utilities|String|ToString(Integer) (Variables|/Game/FirstPersonBP/Blueprints/FirstPersonGameMode.FirstPersonGameMode_C|GetPoint _gmref))))))

(event Custom|Down
  (Utilities|FlowControl|DoOnce false
    (:Completed
      (Effects|SpawnEmitteratLocation "/Game/StarterContent/Particles/P_Explosion.P_Explosion" (Transformation|GetWorldLocation (Variables|Default|GetDefaultSceneRoot)))
      ;[1 1 1] TargetRotation set
      (bind _newtrack_0 (Timeline|Timeline_0 ReverseFromEnd)
        (:Update
          (Transformation|SetRelativeRotation (Variables|Default|GetScene) (Math|Rotator|Lerp(Rotator) "90.000000,0.000000, 0" "0.000000,0.000000,0.000000" _newtrack_0) false false))
        (:Sound
          (Audio|PlaySoundatLocation "/Game/SoundEffect/S_Piston.S_Piston" (Transformation|GetActorLocation (Game|Player|GetPlayerPawn 0)) "0, 0, 0" 1.0 1.0 0.0 0 0 0))))))

(event Custom|Fight
  ;[1 1 1] TargetRotation set
  (bind _newtrack_0 (Timeline|Timeline_0 Play)
    (:Update
      (Transformation|SetRelativeRotation (Variables|Default|GetScene) (Math|Rotator|Lerp(Rotator) "90.000000,0.000000, 0" "0.000000,0.000000,0.000000" _newtrack_0) false false))
    (:Sound
      (Audio|PlaySoundatLocation "/Game/SoundEffect/S_Piston.S_Piston" (Transformation|GetActorLocation (Game|Player|GetPlayerPawn 0)) "0, 0, 0" 1.0 1.0 0.0 0 0 0))))

(event EventBeginPlay
  (bind _asfirst_person_game_mode (Utilities|Casting|CastToFirstPersonGameMode (Game|GetGameMode)))
  (Variables|Default|SetGMRef _asfirst_person_game_mode))

(fn ConstructionScript)